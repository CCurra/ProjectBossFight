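; BaseBoss_BP is a base boss Blueprint for AI pawns that provides hit-point tracking.
; BeginPlay calls Heal, which sets current hit points to the maximum.
; TakeDamage subtracts incoming damage and calls Die when hit points reach zero or below.
; Die is an empty stub, so the base itself has no death behavior.
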(event EventBeginPlay
  (CallFunction|Heal))

(fn ConstructionScript)

(fn TakeDamage
  (params (DamageTaken :type Integer))
  (bind _output_get (Variables|Default|SetCurrentHitPoints (- (Variables|Default|GetCurrentHitPoints) DamageTaken)))
  (if (<= _output_get 0)
    (CallFunction|Die)))

(fn Die)

(fn Heal
  (Variables|Default|SetCurrentHitPoints (Variables|Default|GetMaxHitPoints)))