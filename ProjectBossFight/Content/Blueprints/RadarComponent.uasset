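; RadarComponent is an actor component that makes its owning actor show up on the player's radar.
; On BeginPlay it casts the first player controller's HUD to RadarHUD and registers the owner with it.
; On EndPlay it removes the owner from that HUD, after checking that the player controller is still valid.
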(event EventBeginPlay
  (bind _asradar_hud (Utilities|Casting|CastToRadarHUD (HUD|GetHUD (Game|GetPlayerController 0))))
  (Default|AddtoRadar _asradar_hud (Components|GetOwner)))

(event EventEndPlay
  (params (EndPlayReason :type EEndPlayReason%20Enum :default "Destroyed"))
  (bind _returnvalue (Game|GetPlayerController 0))
  (if (Utilities|IsValid _returnvalue)
    (bind _asradar_hud (Utilities|Casting|CastToRadarHUD (HUD|GetHUD _returnvalue)))
    (Default|RemovefromRadar _asradar_hud (Components|GetOwner))))