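; Laser wall turret that fires pairs of TestProjectile actors while the player is within attack range.
; AggroRange sets the InRange flag from player distance, and Rotation smoothly aims the top mesh at the player, though neither is called in this graph.
; Shoot starts at BeginPlay and re-calls itself through retriggerable delays, spawning zero-damage projectiles at two laser sockets or polling while out of range.
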(event Custom|Rotation
  (bind _returnvalue (Game|GetPlayerCharacter 0))
  (bind _turret_top_staticmesh (Variables|Default|GetTurret_Top_StaticMesh))
  (bind _returnvalue_2 (Transformation|GetWorldLocation _turret_top_staticmesh))
  (bind _returnvalue_3 (Transformation|GetActorLocation _returnvalue))
  (bind _returnvalue_4 (Math|Rotator|FindLookatRotation _returnvalue_2 _returnvalue_3))
  (bind (_roll _pitch _yaw) (Math|Rotator|BreakRotator _returnvalue_4))
  (if (Variables|Default|GetInRange)
    (Transformation|SetWorldRotation (Variables|Default|GetTurret_Top_StaticMesh) (Math|Interpolation|RInterpTo (Transformation|GetWorldRotation (Variables|Default|GetTurret_Top_StaticMesh)) (Math|Rotator|MakeRotator 0.0 _pitch _yaw) (Variables|Default|GetDeltaTime) (Variables|Default|GetRotationSpeed)) false false)))

(event Custom|AggroRange
  (if (< (Transformation|GetDistanceTo self (Game|GetPlayerCharacter 0)) (Variables|Default|GetAttackRange))
    (Variables|Default|SetInRange true)
    (else
      (Variables|Default|SetInRange false))))

(event Custom|Shoot
  (if (Variables|Default|GetInRange)
    (Game|SpawnActorfromClass "/Game/ThirdPersonBP/Blueprints/Pawns/Enemies/Projectiles/TestProjectile.TestProjectile_C" (Transformation|GetSocketTransform (Variables|Default|GetTurret_Top_StaticMesh) "Laser_1" "RTS_World") "Undefined" 0 0 0)
    (Game|SpawnActorfromClass "/Game/ThirdPersonBP/Blueprints/Pawns/Enemies/Projectiles/TestProjectile.TestProjectile_C" (Transformation|GetSocketTransform (Variables|Default|GetTurret_Top_StaticMesh) "Laser_2" "RTS_World") "Undefined" 0 0 0)
    (Utilities|FlowControl|RetriggerableDelay (Variables|Default|GetFireRate))
    (CallFunction|Shoot)
    (else
      (Utilities|FlowControl|RetriggerableDelay 0.2)
      (CallFunction|Shoot))))

(event EventBeginPlay
  (CallFunction|Shoot))

(event EventTick
  (params (DeltaSeconds :type Float%20%28single-precision%29))
  (Variables|Default|SetDeltaTime DeltaSeconds))

(fn ConstructionScript)